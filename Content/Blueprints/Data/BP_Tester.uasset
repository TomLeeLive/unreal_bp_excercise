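; BP_Tester is a test actor that prints base health values from the player data table (플레이어데이터).
; On BeginPlay it counts the table's row names, then looks up each row by using the loop index, starting at 1, as the row name.
; Each row found has its 기본체력 (base health) field printed, so the lookup relies on sequentially numbered row names.
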(event `self.ReceiveBeginPlay`
  (bind _outrownames (`DataTableFunctionLibrary.GetDataTableRowNames` (`self.플레이어데이터`)))
  (for _index (range 1 (+ (`KismetArrayLibrary.Array_Length` _outrownames) 1))
    (bind _returnvalue (`|GetDataTableRow` (`self.플레이어데이터`) (`KismetStringLibrary.Conv_StringToName` (`KismetStringLibrary.Conv_IntToString` _index)))
      (:`then`
        (`KismetSystemLibrary.PrintString` (`KismetStringLibrary.Conv_DoubleToString` (`.기본체력_2_8D9B240342E88C2478EC0FA626EA469C` (break `/Game/Blueprints/Data/BP_SPlayerData` _returnvalue))))))))

(fn `UserConstructionScript`)