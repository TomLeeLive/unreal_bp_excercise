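; BP_Diablo is a playable character Blueprint that handles axis-driven movement and a jump input.
; Each Tick points the controller's rotation along the UpDown/LeftRight vector, then adds full-scale movement along the controller's forward vector.
; The input-check function (입력확인) tests for non-zero axes but has no effect, so movement input applies even when idle.
; Pressing Jump only sets the state enum 현재상태블프.
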(event `self.ReceiveTick`
  (params (DeltaSeconds :type "Float (single-precision)"))
  ;[1 1 1] 캐릭터 이동
  (if (or (!= (`self.GetInputAxisValue`) 0.0) (!= (`self.GetInputAxisValue`) 0.0))
    (`Controller.SetControlRotation` (`self.GetController`) (`KismetMathLibrary.MakeRotFromX` (`KismetMathLibrary.MakeVector` (`self.GetInputAxisValue`) (`self.GetInputAxisValue`))))
    (`self.AddMovementInput` (`self.GetActorForwardVector` (`self.GetController`)))))

(event `InputAction|Jump`
  (params (Key :type "Key Structure"))
  (:`Pressed`
    (set `self.현재상태_블프` "NewEnumerator1")))

(fn `UserConstructionScript`)