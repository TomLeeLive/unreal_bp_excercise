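; BP_PlayerData tracks the player's experience and level against the 플레이어데이터 data table.
; Gaining experience triggers a row-by-row scan from level 1 until required experience exceeds the current total, setting the level one below.
; When the level-up check passes, it calls 레벨업 on the BP_Diablo player pawn.
; Helpers fetch level rows, compute experience-gauge progress and derive max level from the row count.
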(event `경험치획득`
  (params (`획득경험치` :type Integer))
  ;[1 1 1] 경험치 획득
  (set `self.경험치` (+ (`self.경험치`) `획득경험치`))
  (`self.레벨확인`))

(event `레벨확인`
  (bind `_루프인덱스` (`self.루프인덱스`))
  ;[1 1 1] 레벨확인
  (set `self.예전레벨` (`self.현재레벨`))
  (set `self.루프인덱스` 0)
  (set `self.루프실행여부` true)
  (`|ExecutionSequence`
    (:`then_0`
      (while (`self.루프실행여부`)
        (`/Engine/EditorBlueprintResources/StandardMacros.IncrementInt` `_루프인덱스`
          (:`  `
            (bind _returnvalue (`|GetDataTableRow` (`self.플레이어데이터`) (`KismetStringLibrary.Conv_StringToName` (`KismetStringLibrary.Conv_IntToString` `_루프인덱스`)))
              (:`then`
                (if (< (`self.경험치`) (`.필요경험치_7_055E21CF4974F11F423756AFD186F3C9` (break `/Game/Blueprints/Data/BP_SPlayerData` _returnvalue)))
                  (set `self.루프실행여부` false))))))))
    (:`then_1`
      (set `self.현재레벨` (- (`self.루프인덱스`) 1))
      (if (and (!= (`self.예전레벨`) -1) (!= (`self.예전레벨`) (`self.현재레벨`)))
        (`self.레벨 업`)))))

(event `레벨 업`
  ;[1 1 1] 레벨업
  (bind _asbp_diablo (cast `/Game/Blueprints/Character/BP_Diablo` (`GameplayStatics.GetPlayerPawn` 0)))
  (`/Game/Blueprints/Character/BP_Diablo.레벨업` _asbp_diablo))

(event `최고레벨값설정`
  ;[1 1 1] 최고 레벨 값 설정
  (bind _outrownames (`DataTableFunctionLibrary.GetDataTableRowNames` (`self.플레이어데이터`)))
  (set `self.최고레벨값` (`KismetArrayLibrary.Array_Length` _outrownames)))

(fn `경험치게이지구하기`
  (returns (`경험치게이지` :type "Float (double-precision)"))
  (bind (`_레벨데이터_기본체력` `_레벨데이터_공격력` `_레벨데이터_필요경험치`) (break `/Game/Blueprints/Data/BP_SPlayerData` (`self.레벨데이터`)))
  (bind (`_레벨데이터_기본체력_2` `_레벨데이터_공격력_2` `_레벨데이터_필요경험치_2`) (break `/Game/Blueprints/Data/BP_SPlayerData` (`self.레벨데이터`)))
  (bind `_플레이어레벨` (`self.레벨데이터구하기` (+ (`self.현재레벨`) 1)))
  (return (/ (`KismetMathLibrary.Conv_IntToDouble` (- (`self.경험치`) `_레벨데이터_필요경험치_2`)) (`KismetMathLibrary.Conv_IntToDouble` (- (`.필요경험치_7_055E21CF4974F11F423756AFD186F3C9` (break `/Game/Blueprints/Data/BP_SPlayerData` `_플레이어레벨`)) `_레벨데이터_필요경험치`)))))

(fn `레벨데이터구하기`
  (params (`레벨` :type Integer))
  (returns (`플레이어레벨` :type "/Game/Blueprints/Data/BP_SPlayerData Structure"))
  (bind _returnvalue (`|GetDataTableRow` (`self.플레이어데이터`) (`KismetStringLibrary.Conv_StringToName` (`KismetStringLibrary.Conv_IntToString` `레벨`)))
    (:`then`
      (return _returnvalue))))