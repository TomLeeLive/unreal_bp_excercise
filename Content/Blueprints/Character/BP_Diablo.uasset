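; BP_Diablo is a character Blueprint with directional movement and a melee attack.
; Each Tick, the 입력확인 input check gates turning the controller toward the input axes and moving along its forward vector.
; Attack events toggle a state enum, apply a forward dash impulse, or sphere-trace ahead for Pawns and damage the one hit, with debug drawing left on.
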(event `self.ReceiveTick`
  (params (DeltaSeconds :type "Float (single-precision)"))
  ;[1 1 1] 캐릭터 이동
  (if (or (!= (`self.GetInputAxisValue`) 0.0) (!= (`self.GetInputAxisValue`) 0.0))
    (`Controller.SetControlRotation` (`self.GetController`) (`KismetMathLibrary.MakeRotFromX` (`KismetMathLibrary.MakeVector` (`self.GetInputAxisValue`) (`self.GetInputAxisValue`))))
    (`self.AddMovementInput` (`self.GetActorForwardVector` (`self.GetController`)))))

(event `InputAction|Jump`
  (params (Key :type "Key Structure")))

(event `공격종료`
  ;[1 1 1] 공격종료
  (set `self.현재상태_블프` "NewEnumerator0"))

(event `공격시작`
  (set `self.현재상태_블프` "NewEnumerator1"))

(event `공격대시`
  (`CharacterMovementComponent.AddImpulse` (`self.CharacterMovement`) (* (`self.GetActorForwardVector`) (`self.대시파워`)) true))

(event `공격판정`
  (bind _returnvalue (`self.K2_GetActorLocation`))
  (bind (_outhit _returnvalue_2) (`KismetSystemLibrary.SphereTraceSingleForObjects` :`Start` _returnvalue :`End` (+ _returnvalue (* (`self.GetActorForwardVector`) 200.0)) :`Radius` 60.0 :`ObjectTypes` (`|MakeArray` "ObjectTypeQuery3" :!type "EObjectTypeQuery Enum") :`DrawDebugType` "ForDuration"))
  (if _returnvalue_2
    (`GameplayStatics.ApplyDamage` (`.HitActor` (`GameplayStatics.BreakHitResult` _outhit)) 30.0 (`self.GetController`) self)))

(fn `UserConstructionScript`)