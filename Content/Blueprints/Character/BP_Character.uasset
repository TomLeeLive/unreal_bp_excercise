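; BP_Character is a controllable character that moves forward and back, jumps and turns.
; The UpDown axis drives movement along the actor's forward vector, the Jump action triggers a jump, and the Drag axis adds controller yaw.
; M and F switch views by reattaching the single Camera to FirstSpringArm or ThirdSpringArm, respectively.
; Leftover manual offset and rotation nodes are unconnected and never run.
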(event `InputAxis|UpDown`
  (params (AxisValue :type "Float (single-precision)"))
  ;[1 1 1] 캐릭터 앞뒤 이동
  (`self.AddMovementInput` (`self.GetActorForwardVector`) AxisValue))

(event `InputAction|Jump`
  (params (Key :type "Key Structure"))
  ;[1 1 1] 점프
  (:`Pressed`
    (`self.Jump`)))

(event `InputAxis|Drag`
  (params (AxisValue :type "Float (single-precision)"))
  ;[1 1 1] 캐릭터회전
  (`self.AddControllerYawInput` AxisValue))

(event `Key|M`
  (params (Key :type "Key Structure"))
  (:`Pressed`
    (`SceneComponent.K2_AttachToComponent` (`self.Camera`) (`self.FirstSpringArm`) "None" "KeepRelative" "KeepRelative" "KeepRelative" true)))

(event `Key|F`
  (params (Key :type "Key Structure"))
  (:`Pressed`
    (`SceneComponent.K2_AttachToComponent` (`self.Camera`) (`self.ThirdSpringArm`) "None" "KeepRelative" "KeepRelative" "KeepRelative" true)))

(fn `UserConstructionScript`)