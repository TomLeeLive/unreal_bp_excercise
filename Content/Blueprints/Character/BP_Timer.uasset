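; BP_Timer is a reusable count-up timer that signals when elapsed time reaches a target.
; It does not tick itself: 시간업데이트 receives delta time, adds it to elapsed time clamped at the target, then checks expiry.
; On expiry it calls the 시간만료이벤트 dispatcher, which repeats on every later update until 초기화 zeroes elapsed time.
; Other functions set the target and return elapsed time.
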(fn `경과시간확인`
  (returns (`경과시간` :type "Float (double-precision)"))
  (return (`self.경과시간`)))

(fn `목표시간설정`
  (params (`목표시간` :type "Float (double-precision)"))
  (set `self.목표시간` `목표시간`))

(fn `시간만료확인`
  (returns (`시간만료` :type Boolean))
  (return (>= (`self.경과시간`) (`self.목표시간`))))

(fn `시간업데이트`
  (params (`델타타임` :type "Float (double-precision)"))
  (set `self.경과시간` (`KismetMathLibrary.FMin` (+ (`self.경과시간`) `델타타임`) (`self.목표시간`)))
  (bind `_시간만료` (`self.시간만료확인`))
  (if `_시간만료`
    (`self.시간만료이벤트`)))

(fn `초기화`
  (set `self.경과시간` 0.0))