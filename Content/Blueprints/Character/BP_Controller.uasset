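; Player controller Blueprint that creates the main HUD widget (UMG_Main) and manages a five-second skill cooldown.
; 스킬쿨타임시작 starts the cooldown and shows the radial or fill effect image, while 스킬가능여부확인 reports whether the skill is usable.
; Tick advances BPTimer and writes the remaining fraction to the effect's dynamic material parameter "퍼센트".
; BPTimer's expiry event resets the timer, clears the cooldown flag and hides the effect.
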(event `self.ReceiveBeginPlay`
  (bind _returnvalue (`|CreateWidget` "/Game/UMG/UMG_Main.UMG_Main_C"))
  (bind _output_get (set `self.메인위젯` _returnvalue))
  (`UserWidget.AddToViewport` _output_get 0)
  (`/Game/Blueprints/Character/BP_Timer.목표시간설정` (`self.BP_Timer`) 5.0)
  (add `/Game/Blueprints/Character/BP_Timer.시간만료이벤트` (`self.BP_Timer`) (delegate `쿨타임초기화`)))

(event `쿨타임초기화`
  (`/Game/Blueprints/Character/BP_Timer.초기화` (`self.BP_Timer`))
  (set `self.스킬쿨타임여부` false)
  (`Widget.SetVisibility` (`/Game/UMG/UMG_Main.쿨타임효과` (`self.메인위젯`)) "Hidden"))

(event `self.ReceiveTick`
  (params (DeltaSeconds :type "Float (single-precision)"))
  (`self.스킬쿨타임재생`))

(fn `UserConstructionScript`)

(fn `스킬가능여부확인`
  (returns (`스킬가능한지` :type Boolean))
  (return (not (`self.스킬쿨타임여부`))))

(fn `스킬쿨타임시작`
  (set `self.스킬쿨타임여부` true)
  (bind _returnvalue (`Image.GetDynamicMaterial` (`/Game/UMG/UMG_Main.쿨타임효과` (`self.메인위젯`))))
  (`MaterialInstanceDynamic.SetScalarParameterValue` _returnvalue "퍼센트" 1.0)
  (set `self.쿨타임값` 1.0)
  (`Widget.SetVisibility` (`/Game/UMG/UMG_Main.쿨타임효과` (`self.메인위젯`)) "Visible"))

(fn `스킬쿨타임재생`
  (if (`self.스킬쿨타임여부`)
    (`/Game/Blueprints/Character/BP_Timer.시간업데이트` (`self.BP_Timer`) (`GameplayStatics.GetWorldDeltaSeconds`))
    (bind `_경과시간` (`/Game/Blueprints/Character/BP_Timer.경과시간확인` (`self.BP_Timer`)))
    (set `self.쿨타임값` (/ (- 5.0 `_경과시간`) 5.0))
    (bind _returnvalue (`Image.GetDynamicMaterial` (`/Game/UMG/UMG_Main.쿨타임효과` (`self.메인위젯`))))
    (`MaterialInstanceDynamic.SetScalarParameterValue` _returnvalue "퍼센트" (`self.쿨타임값`))))