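; Bear enemy that hunts BP_Diablo through a peace/chase/attack/death state machine, which sets walk speed and mirrors the state to the AI Blackboard.
; PawnSensing starts the chase, and Tick returns to peace beyond sight radius or, while attacking, on a specific player state.
; A toggleable collision deals melee damage; entering attack is left to external logic.
; Damage updates the HP widget and plays a material tint, or at zero health triggers death and timed removal.
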(event `상태변경`
  (params (`몬스터상태` :type "/Game/Blueprints/Monster/EMonsterState Enum" :default "NewEnumerator0"))
  (bind _charactermovement (`self.CharacterMovement`))
  (if (`|EnumInequality` (`self.몬스터상태_블프`) "NewEnumerator3")
    (set `self.몬스터상태_블프` `몬스터상태`)
    (`BlackboardComponent.SetValueAsEnum` (`AIBlueprintHelperLibrary.GetBlackboard` (`self.GetController`)) (`self.몬스터상태키`) (`self.몬스터상태_블프`))
    (switch `/Game/Blueprints/Monster/EMonsterState` (`self.몬스터상태_블프`)
      (:`NewEnumerator0`
        (set `CharacterMovementComponent.MaxWalkSpeed` 300.0 _charactermovement))
      (:`NewEnumerator1`
        (set `CharacterMovementComponent.MaxWalkSpeed` 500.0 _charactermovement))
      (:`NewEnumerator2`
        (set `CharacterMovementComponent.MaxWalkSpeed` 0.0 _charactermovement :!label _label))
      (:`NewEnumerator3`
        (goto _label)))))

(event `거리확인`
  (bind _instigator (`self.Instigator`))
  (`/Engine/EditorBlueprintResources/StandardMacros.IsValid` _instigator
    (:`Is Valid`
      (if (> (`self.GetDistanceTo` _instigator) (`PawnSensingComponent.SightRadius` (`self.PawnSensing`)))
        (`self.상태변경` "NewEnumerator0")
        (set `self.Instigator` null)))))

(event `self.ReceiveBeginPlay`
  (set `self.현재체력` (`self.기본체력`))
  (bind _asumg_hudhp (cast `/Game/UMG/UMG_HUDHP` (`WidgetComponent.GetUserWidgetObject` (`self.HPBar`))))
  (set `self.체력바위젯` _asumg_hudhp)
  (`self.상태변경` "NewEnumerator0")
  (`self.공격판정종료`))

(event `평화상태`
  ;[1 1 1] 상태기계
)

(event `self.ReceiveAnyDamage`
  (params (Damage :type "Float (single-precision)") (DamageType :type "DamageType Object Reference") (InstigatedBy :type "Controller Object Reference") (DamageCauser :type "Actor Object Reference"))
  (set `self.현재체력` (- (`self.현재체력`) Damage))
  (`/Game/UMG/UMG_HUDHP.체력 게이지 업데이트` (`self.체력바위젯`) (/ (`self.현재체력`) (`self.기본체력`)))
  (`/Game/UMG/UMG_HUDHP.데미지 텍스트 애님 재생` (`self.체력바위젯`) (`KismetMathLibrary.FTrunc` Damage))
  (if (> (`self.현재체력`) 0.0)
    (bind (_direction `_색상`) (`Timeline|데미지효과` :!via `PlayFromStart`)
      (:`Update`
        (`MeshComponent.SetVectorParameterValueOnMaterials` (`self.Mesh`) "색상" (`KismetMathLibrary.MakeVector` (.x `_색상`)))))
    (else
      (`self.상태변경` "NewEnumerator3")
      (`PrimitiveComponent.SetCollisionEnabled` (`self.CapsuleComponent`) "NoCollision")
      (`self.SetLifeSpan` 5.0))))

(event `쫓아가기상태`
  ;[1 1 1] 상태기계
  (`self.거리확인`))

(event `공격상태`
  ;[1 1 1] 상태기계
  (`/Engine/EditorBlueprintResources/StandardMacros.IsValid` (`self.Instigator`)
    (:`Is Valid`
      (bind _asbp_diablo (cast `/Game/Blueprints/Character/BP_Diablo` (`self.Instigator`)))
      (if (`|EnumEquality` (`/Game/Blueprints/Character/BP_Diablo.현재상태_블프` _asbp_diablo) "NewEnumerator2")
        (`self.상태변경` "NewEnumerator0")))))

(event `죽음`
  (`self.K2_DestroyActor`))

(event `죽음상태`
  ;[1 1 1] 상태기계
)

(event `self.PawnSensing.OnSeePawn`
  (params (Pawn :type "Pawn Object Reference"))
  (switch `/Game/Blueprints/Monster/EMonsterState` (`self.몬스터상태_블프`)
    (:`NewEnumerator0`
      (bind _asbp_diablo (cast `/Game/Blueprints/Character/BP_Diablo` Pawn))
      (if (`|EnumInequality` (`/Game/Blueprints/Character/BP_Diablo.현재상태_블프` _asbp_diablo) "NewEnumerator2")
        (bind _output_get (set `self.Instigator` _asbp_diablo))
        (`BlackboardComponent.SetValueAsObject` (`AIBlueprintHelperLibrary.GetBlackboard` (`self.GetController`)) (`self.목표플레이어키`) _output_get)
        (`self.상태변경` "NewEnumerator1")))))

(event `self.ReceiveTick`
  (params (DeltaSeconds :type "Float (single-precision)"))
  (switch `/Game/Blueprints/Monster/EMonsterState` (`self.몬스터상태_블프`)
    (:`NewEnumerator0`
      (`self.평화상태`))
    (:`NewEnumerator1`
      (`self.쫓아가기상태`))
    (:`NewEnumerator2`
      (`self.공격상태`))))

(event `공격판정시작`
  (`PrimitiveComponent.SetCollisionEnabled` (`self.AttackCollision`) "QueryOnly"))

(event `공격판정종료`
  (`PrimitiveComponent.SetCollisionEnabled` (`self.AttackCollision`) "NoCollision"))

(event `self.AttackCollision.OnComponentBeginOverlap`
  (params (OverlappedComponent :type "PrimitiveComponent Object Reference") (OtherActor :type "Actor Object Reference") (OtherComp :type "PrimitiveComponent Object Reference") (OtherBodyIndex :type Integer) (bFromSweep :type Boolean) (SweepResult :type "HitResult Structure (by ref)"))
  (`GameplayStatics.ApplyDamage` OtherActor 20.0 (`self.GetController`) self))

(fn `UserConstructionScript`)