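; BP_MonsterController is the AI controller that starts a monster's behavior when it possesses a pawn.
; On possess it initializes the BP_MonsterBB blackboard with a wait time, the pawn's current location and a random navigable target point around it.
; It then runs the BP_MonsterBT behavior tree.
; Blackboard keys are addressed through Korean-named key-name variables, and BeginPlay, Tick and the construction script are empty.
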(event `self.OnPossess`
  (params (PossessedPawn :type "Pawn Object Reference"))
  (bind _returnvalue (`self.K2_GetActorLocation` (`self.K2_GetPawn`)))
  (`|ExecutionSequence`
    (:`then_0`
      (`self.UseBlackboard` "/Game/Blueprints/Monster/AI/BP_MonsterBB.BP_MonsterBB")
      (`BlackboardComponent.SetValueAsFloat` (`self.Blackboard`) (`self.대기시간이름`) 3.0)
      (`BlackboardComponent.SetValueAsVector` (`self.Blackboard`) (`self.현재위치이름`) _returnvalue)
      (`BlackboardComponent.SetValueAsVector` (`self.Blackboard`) (`self.목표위치이름`) (`NavigationSystemV1.K2_GetRandomLocationInNavigableRadius` _returnvalue 700.0 null null)))
    (:`then_1`
      (`self.RunBehaviorTree` "/Game/Blueprints/Monster/AI/BP_MonsterBT.BP_MonsterBT"))))

(fn `UserConstructionScript`)